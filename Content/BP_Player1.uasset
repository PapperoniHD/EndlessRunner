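; BP_Player1 is a player character that speeds up over time and automatically fires projectiles, with lives and score widgets added on BeginPlay.
; Tick raises walk speed toward a cap, checks lives, and calls a Delay-throttled projectile spawn at ProjectileSpawner.
; At zero lives it pauses, adds a death screen and immediately opens MainMenu.
; Player index 0 relays IA_Jump2 to the "Player2"-tagged instance, apparently for shared-input local two-player.
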(event Custom|DeathCheck
  (if (<= (Variables|Default|GetLives) 0)
    (Game|SetGamePaused true)
    (bind _returnvalue (UserInterface|CreateWidget "/Game/Blueprints/Widgets/DeathScreen.DeathScreen_C"))
    (UserInterface|Viewport|AddtoViewport _returnvalue 0)
    (Variables|Default|SetDead? true)
    (Game|OpenLevel(byName) "MainMenu")))

(event Custom|SpawnProjectile
  (Utilities|FlowControl|Delay (Variables|Default|GetProjectileSpawnTime))
  (Game|SpawnActorfromClass "/Game/Blueprints/Projectile.Projectile_C" (Transformation|GetWorldTransform (Variables|Default|GetProjectileSpawner)) "Undefined" 0 0))

(event Input|EnhancedActionEvents|EnhancedInputActionIA_Jump2
  (params (ActionValue :type Boolean) (ElapsedSeconds :type Float%20%28double-precision%29) (TriggeredSeconds :type Float%20%28double-precision%29) (InputAction :type Input%20Action%20Object%20Reference :default "/Game/Input/IA_Jump2.IA_Jump2"))
  (:Triggered
    (if (== (Variables|Default|GetPlayerIndex) 0)
      (bind _outactors (Actor|GetAllActorswithTag "Player2"))
      (bind _asbp_player_1 (Utilities|Casting|CastToBP_Player1 (Utilities|Array|Get(acopy) _outactors)))
      (Character|Jump _asbp_player_1))))

(event EventBeginPlay
  (bind _returnvalue (UserInterface|CreateWidget "/Game/Blueprints/Widgets/P1Lives.P1Lives_C"))
  (UserInterface|Viewport|AddtoViewport _returnvalue 0)
  (bind _returnvalue_2 (UserInterface|CreateWidget "/Game/Blueprints/Widgets/P1Score.P1Score_C"))
  (UserInterface|Viewport|AddtoViewport _returnvalue_2 0)
  (Variables|Default|SetDead? false)
  (if (== (Variables|Default|GetPlayerIndex) 0)
    _))

(event Collision|EventActorBeginOverlap
  (params (OtherActor :type Actor%20Object%20Reference)))

(event EventTick
  (params (DeltaSeconds :type Float%20%28single-precision%29))
  (bind _charactermovement (Variables|Character|GetCharacterMovement))
  (CallFunction|DeathCheck)
  (CallFunction|SpawnProjectile)
  ;[1 1 1] Increase player speed
  (Variables|/Script/Engine.CharacterMovementComponent|SetMaxWalkSpeed _charactermovement (Math|Interpolation|FInterptoConstant (Variables|/Script/Engine.CharacterMovementComponent|GetMaxWalkSpeed _charactermovement) 5e+03 DeltaSeconds 1e+01)))

(fn ConstructionScript)