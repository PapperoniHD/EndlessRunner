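; MapPiece_BP is a self-chaining level segment that builds the map as BP_Player1 moves through it.
; When the player overlaps Spawnbox, it spawns another MapPiece_BP at the ArrowEnd transform, with no guard against repeat spawns.
; DeathBox teleports the player to the piece's SpawnPoint and deducts a life.
; Tick destroys the piece once the player is too far from ArrowEnd in any direction.
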(event OnComponentBeginOverlap(Spawnbox)
  (params (OverlappedComponent :type Primitive%20Component%20Object%20Reference) (OtherActor :type Actor%20Object%20Reference) (OtherComp :type Primitive%20Component%20Object%20Reference) (OtherBodyIndex :type Integer) (bFromSweep :type Boolean) (SweepResult :type Hit%20Result%20Structure%20%28by%20ref%29))
  (Utilities|Casting|CastToBP_Player1 OtherActor)
  (Game|SpawnActorfromClass "MapPiece_BP_C" (Transformation|GetWorldTransform (Variables|Default|GetArrowEnd)) "Undefined" 0 0))

(event OnComponentBeginOverlap(DeathBox)
  (params (OverlappedComponent :type Primitive%20Component%20Object%20Reference) (OtherActor :type Actor%20Object%20Reference) (OtherComp :type Primitive%20Component%20Object%20Reference) (OtherBodyIndex :type Integer) (bFromSweep :type Boolean) (SweepResult :type Hit%20Result%20Structure%20%28by%20ref%29))
  (bind _asbp_player_1 (Utilities|Casting|CastToBP_Player1 OtherActor))
  (Transformation|Teleport _asbp_player_1 (Transformation|GetWorldLocation (Variables|Default|GetSpawnPoint)) "0, 0, 0")
  (Variables|/Script/EndlessRunnerFG.Player1CPP|SetLives _asbp_player_1 (- (Variables|/Script/EndlessRunnerFG.Player1CPP|GetLives _asbp_player_1) 1)))

(event EventBeginPlay
  (bind _returnvalue (Actor|GetActorOfClass "/Game/BP_Player1.BP_Player1_C"))
  (Variables|Default|SetPlayerREF _returnvalue))

(event Collision|EventActorBeginOverlap
  (params (OtherActor :type Actor%20Object%20Reference)))

(event EventTick
  (params (DeltaSeconds :type Float%20%28single-precision%29))
  (if (> (Math|Vector|Distance(Vector) (Transformation|GetWorldLocation (Variables|Default|GetArrowEnd)) (Transformation|GetWorldLocation (Variables|/Script/Engine.Character|GetCapsuleComponent (Variables|Default|GetPlayerREF)))) 5e+03)
    (Development|PrintText "Destroyed Platform")
    (Actor|DestroyActor)))

(fn ConstructionScript)