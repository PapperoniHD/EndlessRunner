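; Player 1 character for what appears to be an auto-running game, with Space to jump and HUD widgets for lives and score created on BeginPlay.
; Tick pushes constant movement along negative Y and increments Score every frame, so scoring depends on frame rate.
; A Delay on Tick acts as a repeating timer, spawning a Projectile at the ProjectileSpawner transform after each ProjectileSpawnTime interval.
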(event EventBeginPlay
  (bind _returnvalue (UserInterface|CreateWidget "/Game/Blueprints/Widgets/P1Lives.P1Lives_C"))
  (UserInterface|Viewport|AddtoViewport _returnvalue 0)
  (bind _returnvalue_2 (UserInterface|CreateWidget "/Game/Blueprints/Widgets/P1Score.P1Score_C"))
  (UserInterface|Viewport|AddtoViewport _returnvalue_2 0))

(event Collision|EventActorBeginOverlap
  (params (OtherActor :type Actor%20Object%20Reference)))

(event EventTick
  (params (DeltaSeconds :type Float%20%28single-precision%29))
  (Utilities|FlowControl|Sequence
    (:then_0
      (Pawn|Input|AddMovementInput "0.000000,-1.000000,0.000000" 1.0 false))
    (:then_1
      (Variables|Default|SetScore (+ (Variables|Default|GetScore) 1)))
    (:then_2
      (Utilities|FlowControl|Delay (Variables|Default|GetProjectileSpawnTime))
      (Game|SpawnActorfromClass "/Game/Blueprints/Projectile.Projectile_C" (Transformation|GetWorldTransform (Variables|Default|GetProjectileSpawner)) "Undefined" 0 0))))

(event Input|KeyboardEvents|SpaceBar
  (params (Key :type Key%20Structure :default "None"))
  (:Pressed
    (Character|Jump)))

(fn ConstructionScript)