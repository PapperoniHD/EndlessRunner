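; Score manager Blueprint that tracks the game's high score.
; Every Tick it casts the game instance to GameInstanceBP and raises its HighScore whenever Score exceeds it.
; Unconnected load and save chains for a SaveGameHS object never run, and the save chain never writes to a slot, so this Blueprint does not persist the high score to disk.
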(event EventBeginPlay)

(event Collision|EventActorBeginOverlap
  (params (OtherActor :type Actor%20Object%20Reference)))

(event EventTick
  (params (DeltaSeconds :type Float%20%28single-precision%29))
  (bind _score (Variables|Default|GetScore))
  (bind _asgame_instance_bp (Utilities|Casting|CastToGameInstanceBP (Game|GetGameInstance)))
  (if (> _score (Variables|/Game/GameInstanceBP.GameInstanceBP_C|GetHigh%20Score _asgame_instance_bp))
    (Variables|/Game/GameInstanceBP.GameInstanceBP_C|SetHigh%20Score _asgame_instance_bp _score)))

(fn ConstructionScript)